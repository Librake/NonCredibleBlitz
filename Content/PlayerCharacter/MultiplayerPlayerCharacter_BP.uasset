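; Multiplayer player character Blueprint that handles two-slot gun firing, arms animation, HUD, death and respawn.
; Fire routes to the active weapon, with a timeline repeating Fire for full-auto guns.
; Weapon visibility, death ragdoll and random-point respawn pass through Server-to-Multicast event chains, while widgets use Client events.
; Camera transform relays follow the same pattern, but their driving timeline is never started here.
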(event Custom|Client%20Get%20Camera%20Location
  (bind _player_camera (Variables|Default|GetPlayer%20Camera))
  ;[0 0 0] Get Camera Location
  (bind _output_get (Variables|Default|SetCameraLocation (Transformation|GetWorldLocation _player_camera)))
  (bind _output_get_2 (Variables|Default|SetCameraRotation (Transformation|GetWorldRotation _player_camera)))
  (CallFunction|ServerGetCameraLocation _output_get _output_get_2))

(event Custom|Server%20Get%20Camera%20Location
  (params (Camera%20Location :type Vector) (Camera%20Rotation :type Rotator))
  ;[0 0 0] Get Camera Location
  (CallFunction|MulticastGetCameraLocation Camera%20Location Camera%20Rotation))

(event Custom|ServerSetWeapon1Hidden%20BP
  (params (Hidden :type Boolean))
  ;[0 0 0] Guns
  (CallFunction|MulticastSetWeapon1HiddenBP Hidden))

(event Custom|MulticastSetWeapon1Hidden%20BP
  (params (Hidden :type Boolean))
  (bind _weapon1 (Variables|Default|GetWeapon1))
  ;[0 0 0] Guns
  (Utilities|IsValid _weapon1
    (:Is%20Valid
      (Rendering|SetActorHiddenInGame _weapon1 Hidden)
      (bind _asmultiplayer_gun_master_class_bp (Utilities|Casting|CastToMultiplayerGunMasterClass_BP _weapon1))
      (Default|ServerSetWeaponHidden _asmultiplayer_gun_master_class_bp Hidden))))

(event Custom|ServerSetWeapon2Hidden%20BP
  (params (Hidden :type Boolean))
  ;[0 0 0] Guns
  (CallFunction|MulticastSetWeapon2HiddenBP Hidden))

(event Custom|MulticastSetWeapon2Hidden%20BP
  (params (Hidden :type Boolean))
  (bind _weapon2 (Variables|Default|GetWeapon2))
  ;[0 0 0] Guns
  (Utilities|IsValid _weapon2
    (:Is%20Valid
      (Rendering|SetActorHiddenInGame _weapon2 Hidden)
      (bind _asmultiplayer_gun_master_class_bp (Utilities|Casting|CastToMultiplayerGunMasterClass_BP _weapon2))
      (Default|ServerSetWeaponHidden _asmultiplayer_gun_master_class_bp Hidden))))

(event Custom|Client%20Fire%20Montage%20Play
  (bind _weaponbeingused (Variables|Default|GetWeaponBeingUsed))
  (bind _arms_mesh (Variables|Default|GetArms%20Mesh))
  (bind _returnvalue (Components|SkeletalMesh|GetAnimInstance _arms_mesh))
  ;[0 0 0] Guns
  (if (== _weaponbeingused 1)
    (bind _asmultiplayer_gun_master_class_bp (Utilities|Casting|CastToMultiplayerGunMasterClass_BP (Variables|Default|GetWeapon1)))
    (Utilities|IsValid (Variables|/Script/MultiplayerShooterPlugin.MultiplayerGunMasterClass|GetFireAnimationMontage _asmultiplayer_gun_master_class_bp)
      (:Is%20Valid
        (Animation|Montage|MontagePlay _returnvalue (Variables|/Script/MultiplayerShooterPlugin.MultiplayerGunMasterClass|GetFireAnimationMontage _asmultiplayer_gun_master_class_bp) 1.0 "MontageLength" 0.0 true)))
    (elif (== _weaponbeingused 2)
      (bind _asmultiplayer_gun_master_class_bp_2 (Utilities|Casting|CastToMultiplayerGunMasterClass_BP (Variables|Default|GetWeapon2)))
      (Utilities|IsValid (Variables|/Script/MultiplayerShooterPlugin.MultiplayerGunMasterClass|GetFireAnimationMontage _asmultiplayer_gun_master_class_bp_2)
        (:Is%20Valid
          (Animation|Montage|MontagePlay _returnvalue (Variables|/Script/MultiplayerShooterPlugin.MultiplayerGunMasterClass|GetFireAnimationMontage _asmultiplayer_gun_master_class_bp_2) 1.0 "MontageLength" 0.0 true))))))

(event Custom|Multicast%20Get%20Camera%20Location
  (params (Camera%20Location :type Vector) (Camera%20Rotation :type Rotator))
  ;[0 0 0] Get Camera Location
  (Variables|Default|SetCameraLocation Camera%20Location)
  (Variables|Default|SetCameraRotation Camera%20Rotation))

(event Custom|Client%20Show%20Default%20HUD
  ;[0 0 0] Default HUD
  (bind _asplayer_controller (Utilities|Casting|CastToPlayerController (Pawn|GetController)))
  (bind _returnvalue (UserInterface|CreateWidget "/Game/UI/DefaultHUD.DefaultHUD_C" _asplayer_controller))
  (UserInterface|Viewport|AddtoViewport _returnvalue 0))

(event Custom|ClientDie%20BP
  ;[0 0 0] Die BP and Respawn BP
  (bind _asplayer_controller (Utilities|Casting|CastToPlayerController (Pawn|GetController)))
  (Viewport|RemoveAllWidgets)
  (bind _returnvalue (UserInterface|CreateWidget "/Game/UI/DeathScreen.DeathScreen_C" _asplayer_controller))
  (UserInterface|Viewport|AddtoViewport _returnvalue 2147483647))

(event Custom|ClientRespawn%20BP
  ;[0 0 0] Die BP and Respawn BP
  (bind _asplayer_controller (Utilities|Casting|CastToPlayerController (Pawn|GetController)))
  (Viewport|RemoveAllWidgets)
  (if (Variables|Default|GetbUseDefaultPluginHUD)
    (bind _returnvalue (UserInterface|CreateWidget "/Game/UI/DefaultHUD.DefaultHUD_C" _asplayer_controller))
    (UserInterface|Viewport|AddtoViewport _returnvalue 0)))

(event Custom|ServerRespawn%20BP
  ;[0 0 0] Die BP and Respawn BP
  (CallFunction|MulticastRespawnBP))

(event Custom|MulticastRespawn%20BP
  (bind _mesh (Variables|Character|GetMesh))
  ;[0 0 0] Die BP and Respawn BP
  (Physics|SetSimulatePhysics _mesh false)
  (Transformation|AttachComponentToComponent _mesh (Variables|Default|GetCapsuleComponent) "None" "KeepWorld" "KeepWorld" "KeepWorld" true)
  (Transformation|SetRelativeLocationAndRotation _mesh "0, 0,-88.000000" "0,-90.000000, 0" false false)
  (Transformation|Teleport (.OutItem (Utilities|Array|Random (Variables|Health|GetRespawnLocations))) "0, 0, 0"))

(event Custom|ServerDie%20BP
  ;[0 0 0] Die BP and Respawn BP
  (CallFunction|MulticastDieBP))

(event Custom|MulticastDie%20BP
  ;[0 0 0] Die BP and Respawn BP
  (Physics|SetSimulatePhysics (Variables|Character|GetMesh) true))

(event EventBeginPlayBP
  ;[0 0 0] Begin Play
  (Variables|Default|SetPlayerBPCamera (Variables|Default|GetPlayer%20Camera))
  (Utilities|FlowControl|Delay 0.5)
  (Class|MultiplayerPlayerCharacter|SetWeapon1HiddenBP false))

(event EventSetPlayerModelforWeaponsBP
  ;[0 0 0] Guns
  (bind _asmultiplayer_gun_master_class_bp (Utilities|Casting|CastToMultiplayerGunMasterClass_BP (Variables|Default|GetWeapon1))
    (:then
      (Variables|/Script/MultiplayerShooterPlugin.MultiplayerGunMasterClass|SetThirdPersonCharacterMesh _asmultiplayer_gun_master_class_bp (Variables|Character|GetMesh)))
    (:CastFailed
      _))
  (bind _asmultiplayer_gun_master_class_bp_2 (Utilities|Casting|CastToMultiplayerGunMasterClass_BP (Variables|Default|GetWeapon2)))
  (Variables|/Script/MultiplayerShooterPlugin.MultiplayerGunMasterClass|SetThirdPersonCharacterMesh _asmultiplayer_gun_master_class_bp_2 (Variables|Character|GetMesh)))

(event EventSetWeapon1HiddenBP
  (params (Hidden :type Boolean))
  ;[0 0 0] Guns
  (CallFunction|ServerSetWeapon1HiddenBP Hidden))

(event EventSetWeapon2HiddenBP
  (params (Hidden :type Boolean))
  ;[0 0 0] Guns
  (CallFunction|ServerSetWeapon2HiddenBP Hidden))

(event EventFireBP
  (bind _weaponbeingused (Variables|Default|GetWeaponBeingUsed))
  ;[0 0 0] Guns
  (if (Variables|Default|GetbCanShoot)
    (if (== _weaponbeingused 1)
      (bind _asmultiplayer_gun_master_class_bp (Utilities|Casting|CastToMultiplayerGunMasterClass_BP (Variables|Default|GetWeapon1)))
      (if (== (Variables|/Script/MultiplayerShooterPlugin.MultiplayerGunMasterClass|GetFireMode _asmultiplayer_gun_master_class_bp) 0)
        (Timeline|Weapon1%20Fire%20Full%20Auto%20Timeline PlayFromStart
          (:Update
            _)))
      (Class|MultiplayerPlayerCharacter|Fire)
      (elif (== _weaponbeingused 2)
        (bind _asmultiplayer_gun_master_class_bp_2 (Utilities|Casting|CastToMultiplayerGunMasterClass_BP (Variables|Default|GetWeapon2)))
        (if (== (Variables|/Script/MultiplayerShooterPlugin.MultiplayerGunMasterClass|GetFireMode _asmultiplayer_gun_master_class_bp_2) 0)
          (Timeline|Weapon2%20Fire%20Full%20Auto%20Timeline PlayFromStart
            (:Update
              _)))
        (Class|MultiplayerPlayerCharacter|Fire)))))

(event EventStopFiringBP
  ;[0 0 0] Guns
  (Audio|Components|Audio|Stop (Variables|Default|GetWeapon1%20Fire%20Full%20Auto%20Timeline)))

(event EventShowDefaultPluginHUDBP
  ;[0 0 0] Default HUD
  (CallFunction|ClientShowDefaultHUD))

(event EventDieBP
  ;[0 0 0] Die BP and Respawn BP
  (CallFunction|ClientDieBP)
  (CallFunction|ServerDieBP))

(event EventRespawnBP
  ;[0 0 0] Die BP and Respawn BP
  (CallFunction|ClientRespawnBP)
  (CallFunction|ServerRespawnBP)
  (Utilities|FlowControl|Delay 0.5)
  (Class|MultiplayerPlayerCharacter|SetWeapon1HiddenBP false))

(event EventPlayArmsAnimationBP
  (params (Animation :type Animation%20Asset%20Object%20Reference) (bLooping :type Boolean))
  ;[0 0 0] Animation
  (Utilities|IsValid Animation
    (:Is%20Valid
      (Components|Animation|PlayAnimation (Variables|Default|GetArms%20Mesh) Animation bLooping))))

(event EventSetArmsAnimationModeBP
  (params (AnimationMode :type EAnimationMode%20Enum :default "AnimationBlueprint"))
  ;[0 0 0] Animation
  (Components|Animation|SetAnimationMode (Variables|Default|GetArms%20Mesh) AnimationMode))

(fn ConstructionScript)