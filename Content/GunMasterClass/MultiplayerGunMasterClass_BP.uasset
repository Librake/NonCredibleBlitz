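; Multiplayer gun master Blueprint handling fire feedback, pickup attachment, weapon visibility and shotgun spread.
; FireBP runs timeline-driven recoil, then authority multicasts montage, sound and muzzle flash and triggers camera shake, while remotes call ServerFireBP, which enters the effects body directly.
; Hit particles, standalone muzzle flashes and hiding relay from server events to multicasts.
; Owner-visibility flags separate first- and third-person meshes and fire flashes.
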(event Custom|ServerFireBP
  (bind _muzzleflashparticle (Variables|Default|GetMuzzleFlashParticle))
  (bind _firesound (Variables|Default|GetFireSound))
  ;[0 0 0] Fire BP
  (bind _asmultiplayer_player_character_bp (Utilities|Casting|CastToMultiplayerPlayerCharacter_BP (Variables|Default|GetOwningPlayer))
    (:then
      (if (Variables|Default|GetbPlayUnrealDefaultArmsAnimation)
        (Default|ClientFireMontagePlay _asmultiplayer_player_character_bp)))
    (:CastFailed
      _))
  (Utilities|IsValid _firesound
    (:Is%20Valid
      (Audio|PlaySoundatLocation _firesound (Transformation|GetWorldLocation (Variables|Default|GetBarrelEndScene)) "0, 0, 0" 1.0 1.0 0.0 0 0 0 0))
    (:Is%20Not%20Valid
      _))
  (Utilities|IsValid _muzzleflashparticle
    (:Is%20Valid
      (bind _returnvalue (Effects|SpawnEmitterAttached _muzzleflashparticle (Variables|Default|GetBarrelEndScene) "None"))
      (Rendering|SetOnlyOwnerSee _returnvalue true :!class /Script/Engine.PrimitiveComponent)
      (bind _returnvalue_2 (Effects|SpawnEmitterAttached _muzzleflashparticle (Variables|Default|GetBarrelEndSceneThirdPerson) "None"))
      (Class|PrimitiveComponent|SetOwnerNoSee _returnvalue_2 true))))

(event Custom|MulticastFireBP
  (bind _muzzleflashparticle (Variables|Default|GetMuzzleFlashParticle))
  (bind _firesound (Variables|Default|GetFireSound))
  ;[0 0 0] Fire BP
  (bind _asmultiplayer_player_character_bp (Utilities|Casting|CastToMultiplayerPlayerCharacter_BP (Variables|Default|GetOwningPlayer))
    (:then
      (if (Variables|Default|GetbPlayUnrealDefaultArmsAnimation)
        (Default|ClientFireMontagePlay _asmultiplayer_player_character_bp)))
    (:CastFailed
      _))
  (Utilities|IsValid _firesound
    (:Is%20Valid
      (Audio|PlaySoundatLocation _firesound (Transformation|GetWorldLocation (Variables|Default|GetBarrelEndScene)) "0, 0, 0" 1.0 1.0 0.0 0 0 0 0))
    (:Is%20Not%20Valid
      _))
  (Utilities|IsValid _muzzleflashparticle
    (:Is%20Valid
      (bind _returnvalue (Effects|SpawnEmitterAttached _muzzleflashparticle (Variables|Default|GetBarrelEndScene) "None"))
      (Rendering|SetOnlyOwnerSee _returnvalue true :!class /Script/Engine.PrimitiveComponent)
      (bind _returnvalue_2 (Effects|SpawnEmitterAttached _muzzleflashparticle (Variables|Default|GetBarrelEndSceneThirdPerson) "None"))
      (Class|PrimitiveComponent|SetOwnerNoSee _returnvalue_2 true))))

(event Custom|Multicast%20Show%20Hit%20Particle
  (params (Selected%20Effect :type Particle%20System%20Object%20Reference) (Location :type Vector))
  ;[0 0 0] Fire BP
  (Utilities|IsValid Selected%20Effect
    (:Is%20Valid
      (Effects|SpawnEmitteratLocation Selected%20Effect Location "0, 0, 0" (Variables|Default|GetHitParticleScale)))))

(event Custom|ServerSetWeaponHidden
  (params (Hidden :type Boolean))
  ;[0 0 0] Set Weapon Hidden
  (CallFunction|MulticastSetWeaponHidden Hidden))

(event Custom|MulticastSetWeaponHidden
  (params (Hidden :type Boolean))
  ;[0 0 0] Set Weapon Hidden
  (Rendering|SetActorHiddenInGame Hidden))

(event Custom|Client%20Play%20Camera%20Shake
  (bind _camera_shake (Variables|CameraShake|GetCamera%20Shake))
  ;[0 0 0] Fire BP
  (if (Utilities|IsValidClass _camera_shake)
    (bind _asmultiplayer_player_character_bp (Utilities|Casting|CastToMultiplayerPlayerCharacter_BP (Variables|Default|GetOwningPlayer)))
    (bind _asplayer_controller (Utilities|Casting|CastToPlayerController (Pawn|GetController _asmultiplayer_player_character_bp)))
    (Game|Feedback|ClientStartCameraShake _asplayer_controller _camera_shake 1.0 "CameraLocal" "0, 0, 0")))

(event Custom|Client%20Fire%20BP
  ;[0 0 0] Fire BP
  (bind _asmultiplayer_player_character_bp (Utilities|Casting|CastToMultiplayerPlayerCharacter_BP (Variables|Default|GetOwningPlayer)))
  (bind _value (Timeline|Recoil%20Interpolation%20Timeline PlayFromStart)
    (:Update
      (Pawn|SetControlRotation (Pawn|GetController _asmultiplayer_player_character_bp) (Math|Rotator|MakeRotator (.roll (Pawn|GetControlRotation (Pawn|GetController _asmultiplayer_player_character_bp) :!class /Script/Engine.Controller)) (Math|Float|MapRangeClamped _value 0.0 1.0 (.pitch (Pawn|GetControlRotation (Pawn|GetController _asmultiplayer_player_character_bp) :!class /Script/Engine.Controller)) (- (.pitch (Pawn|GetControlRotation (Pawn|GetController _asmultiplayer_player_character_bp) :!class /Script/Engine.Controller)) (Variables|Default|GetVerticleRecoil))) (Math|Float|MapRangeClamped _value 0.0 1.0 (.yaw (Pawn|GetControlRotation (Pawn|GetController _asmultiplayer_player_character_bp) :!class /Script/Engine.Controller)) (+ (.yaw (Pawn|GetControlRotation (Pawn|GetController _asmultiplayer_player_character_bp) :!class /Script/Engine.Controller)) (Variables|Default|GetHorizontalRecoil))))))))

(event Custom|Server%20Show%20Muzzle%20Flash%20BP
  ;[0 0 0] Fire BP
  (CallFunction|MulticastShowMuzzleFlashBP))

(event Custom|Multicast%20Show%20Muzzle%20Flash%20BP
  (bind _muzzleflashparticle (Variables|Default|GetMuzzleFlashParticle))
  ;[0 0 0] Fire BP
  (Utilities|IsValid _muzzleflashparticle
    (:Is%20Valid
      (Effects|SpawnEmitterAttached _muzzleflashparticle (Variables|Default|GetBarrelEndScene) "None"))))

(event Custom|Server%20Show%20Hit%20Particle
  (params (Selected%20Effect :type Particle%20System%20Object%20Reference) (Location :type Vector))
  ;[0 0 0] Fire BP
  (CallFunction|MulticastShowHitParticle Selected%20Effect Location))

(event EventFireBP
  ;[0 0 0] Fire BP
  (CallFunction|ClientFireBP)
  (Networking|SwitchHasAuthority
    (:Authority
      (CallFunction|MulticastFireBP)
      (CallFunction|ClientPlayCameraShake))
    (:Remote
      (CallFunction|ServerFireBP))))

(event EventSetThirdPersonBP
  (params (ThirdPerson :type Boolean))
  ;[0 0 0] Third Person
  (Class|PrimitiveComponent|SetOwnerNoSee (Variables|Default|GetGunMesh) ThirdPerson)
  (Class|PrimitiveComponent|SetOwnerNoSee (Variables|Default|GetThirdPersonGunMesh) (not ThirdPerson)))

(event EventSetShotgunFireRotationBP
  ;[0 0 0] Shotguns
  (Variables|Default|SetShotgunFireRotation (Math|Rotator|MakeRotator (.roll (Variables|Default|GetShotgunFireRotation)) (+ (.pitch (Variables|Default|GetShotgunFireRotation)) (Math|Random|RandomFloatinRange (Variables|Default|GetShotgunMinVerticalSpread) (Variables|Default|GetShotgunMaxVerticalSpread))) (+ (.yaw (Variables|Default|GetShotgunFireRotation)) (Math|Random|RandomFloatinRange (Variables|Default|GetShotgunMinHorizontalSpread) (Variables|Default|GetShotgunMaxHorizontalSpread))))))

(event EventShowMuzzleFlashBP
  ;[0 0 0] Fire BP
  (CallFunction|ServerShowMuzzleFlashBP))

(event EventGetPickedUpBP
  ;[0 0 0] Pickup
  (bind _asmultiplayer_player_character_bp (Utilities|Casting|CastToMultiplayerPlayerCharacter_BP (Variables|Default|GetOwningPlayer)))
  (Transformation|AttachComponentToComponent (Variables|/Game/PlayerCharacter/MultiplayerPlayerCharacter_BP.MultiplayerPlayerCharacter_BP_C|GetArms%20Mesh _asmultiplayer_player_character_bp) (Variables|Default|GetSocket) "KeepWorld" "KeepWorld" "KeepWorld" true))

(event EventShowHitParticleBP
  (params (SelectedEffect :type Particle%20System%20Object%20Reference) (Location :type Vector :default "0, 0, 0"))
  ;[0 0 0] Fire BP
  (CallFunction|ServerShowHitParticle SelectedEffect Location))

(fn ConstructionScript)